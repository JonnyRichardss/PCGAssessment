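; Solar system generator actor that builds a procedural star system on BeginPlay from SystemSettings.
; GenAll creates a system template, spawns planet, comet and solar ring actors on a shared orbital plane, then scales and colours the star sphere through a dynamic material.
; RegenAsteroids separately bakes procedural asteroid and ice ball meshes into static mesh assets via temporary dynamic mesh components.
; A disabled debug branch draws orbit limits.
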(event `self.ReceiveBeginPlay`
  (`self.GenAll`))

(fn `GenAll`
  (bind _shape_sphere (`self.Shape_Sphere`))
  (bind _returnvalue (`_JR_SolarSystemGenerator.GenerateSystemTemplate` (`self.SystemSettings`)))
  (`self.Generate` _returnvalue)
  (bind _star (break `SolarSystemSettings` _returnvalue))
  (`SceneComponent.K2_SetWorldTransform` _shape_sphere (`KismetMathLibrary.MakeTransform` (`KismetMathLibrary.MakeVector` 0.0 0.0 (* -50.0 (break `StarSettings` _star))) (struct) (`KismetMathLibrary.Conv_DoubleToVector` (break `StarSettings` _star))) false true)
  (bind _returnvalue_2 (`PrimitiveComponent.CreateDynamicMaterialInstance` _shape_sphere 0 "/Game/sunMat/SunMat.SunMat" "None"))
  (`MaterialInstanceDynamic.SetScalarParameterValue` _returnvalue_2 "NoiseScale" (/ (break `StarSettings` _star) 250000.0))
  (`MaterialInstanceDynamic.SetScalarParameterValue` _returnvalue_2 "Brightness" (`.brightness` (break `StarSettings` _star)))
  (bind _star_2 (break `SolarSystemSettings` _returnvalue))
  (`MaterialInstanceDynamic.SetVectorParameterValue` _returnvalue_2 "MainColour" (`.col1` (break `StarSettings` _star_2)))
  (`MaterialInstanceDynamic.SetVectorParameterValue` _returnvalue_2 "SecondaryColour" (`.col2` (break `StarSettings` _star_2))))

(fn `Generate`
  (params (settings :type "SolarSystemSettings Structure"))
  (bind (_star _planets _solarrings _comets _orbitplane) (break `SolarSystemSettings` settings))
  (bind (_star_2 _planets_2 _solarrings_2 _comets_2 _orbitplane_2) (break `SolarSystemSettings` settings))
  (bind (_star_3 _planets_3 _solarrings_3 _comets_3 _orbitplane_3) (break `SolarSystemSettings` settings))
  (bind _systemsettings (`self.SystemSettings`))
  (bind _generated (`self.Generated`))
  (bind _systemsettings_2 (`self.SystemSettings`))
  (bind _returnvalue (`KismetMathLibrary.Normal` (`KismetMathLibrary.ProjectPointOnToPlane` (`KismetMathLibrary.RandomUnitVector`) (0.0 0.0 0.0) _orbitplane_3)))
  (bind _returnvalue_2 (`KismetMathLibrary.Cross_VectorVector` _orbitplane_3 _returnvalue))
  (set `self.SettingsDBG` settings)
  (for _array_element _generated
    (`self.K2_DestroyActor` _array_element))
  (`KismetArrayLibrary.Array_Clear` _generated)
  (`|ExecutionSequence`
    (:`then_0`
      (for _array_element_2 _planets_2
        (bind _returnvalue_3 (`|SpawnActorFromClass` "/Game/Blueprints/BP_Planet.BP_Planet_C" (`self.GetTransform`) "Undefined" "MultiplyWithRoot" null _array_element_2 _orbitplane_2 null))
        (`KismetArrayLibrary.Array_Add` (`self.Generated`) _returnvalue_3)))
    (:`then_1`
      (for _array_element_3 _comets
        (bind _returnvalue_4 (`|SpawnActorFromClass` "/Game/Blueprints/BP_Comet.BP_Comet_C" (`self.GetTransform`) "Undefined" "MultiplyWithRoot" null _array_element_3 (`.mass` (break `StarSettings` _star)) _orbitplane null))
        (`KismetArrayLibrary.Array_Add` (`self.Generated`) _returnvalue_4)))
    (:`then_2`
      (for _array_element_4 _solarrings
        (bind _returnvalue_5 (`|SpawnActorFromClass` "/Game/Blueprints/BP_PlanetRing.BP_PlanetRing_C" (`self.GetTransform`) "Undefined" "MultiplyWithRoot" null _array_element_4 true _orbitplane null))
        (`KismetArrayLibrary.Array_Add` (`self.Generated`) _returnvalue_5)))
    (:`then_3`
      ; Debug
      (if false
        (`self.Draw2circles` _returnvalue_2 _returnvalue (`.MinOrbit` (break `SolarSystemMetaSettings` _systemsettings_2)) (struct :`G` 0.052337 :`B` 1.0 :`A` 1.0)
          (:`  `
            (`self.Draw2circles` _returnvalue_2 _returnvalue (`.IonMaxDistance` (break `CometMetaSettings` (`.CometSettings` (break `SolarSystemMetaSettings` _systemsettings_2)))) (struct :`R` 1.0 :`B` 0.029831 :`A` 1.0)
              (:`  `
                (`self.Draw2circles` _returnvalue_2 _returnvalue (`.MaxOrbit` (break `SolarSystemMetaSettings` _systemsettings_2)) (struct :`G` 0.037928 :`B` 1.0 :`A` 1.0)
                  (:`  `
                    (`self.Draw2circles` _returnvalue_2 _returnvalue (`.Radius` (break `CometMetaSettings` (`.CometSettings` (break `SolarSystemMetaSettings` _systemsettings_2)))) (struct :`R` 0.885713 :`B` 1.0 :`A` 1.0)
                      (:`  `
                        (`KismetSystemLibrary.DrawDebugSphere` (0.0 0.0 0.0) (* (break `Vector2f` (break `StarMetaSettings` (break `SolarSystemMetaSettings` _systemsettings))) 50.0) 12 (struct :`R` 1.0 :`B` 0.924422 :`A` 1.0) 100000.0 1000.0)
                        (`KismetSystemLibrary.DrawDebugSphere` (0.0 0.0 0.0) (* (`.Y` (break `Vector2f` (break `StarMetaSettings` (break `SolarSystemMetaSettings` _systemsettings)))) 50.0) 12 (struct :`R` 1.0 :`B` 0.924422 :`A` 1.0) 100000.0 1000.0)))))))))))))

(fn `RegenAsteroids`
  (bind _comparray (`self.CompArray`))
  (`|ExecutionSequence`
    (:`then_0`
      (`|ExecutionSequence`
        (:`then_0`
          (`|ExecutionSequence`
            (:`then_0`
              (bind _returnvalue (`self.MakeAst`))
              (`GeometryScriptLibrary_StaticMeshFunctions.CopyMeshToStaticMesh` _returnvalue "/Game/Niagara/Asteroids/Ast1.Ast1" (struct) (struct) true null))
            (:`then_1`
              (bind _returnvalue_2 (`self.MakeAst`))
              (`GeometryScriptLibrary_StaticMeshFunctions.CopyMeshToStaticMesh` _returnvalue_2 "/Game/Niagara/Asteroids/Ast2.Ast2" (struct) (struct) true null))
            (:`then_2`
              (bind _returnvalue_3 (`self.MakeAst`))
              (`GeometryScriptLibrary_StaticMeshFunctions.CopyMeshToStaticMesh` _returnvalue_3 "/Game/Niagara/Asteroids/Ast3.Ast3" (struct) (struct) true null))))
        (:`then_1`
          (`|ExecutionSequence`
            (:`then_0`
              (bind _returnvalue_4 (`self.MakeIceBall`))
              (`GeometryScriptLibrary_StaticMeshFunctions.CopyMeshToStaticMesh` _returnvalue_4 "/Game/Niagara/Asteroids/Ice1.Ice1" (struct) (struct) true null))
            (:`then_1`
              (bind _returnvalue_5 (`self.MakeIceBall`))
              (`GeometryScriptLibrary_StaticMeshFunctions.CopyMeshToStaticMesh` _returnvalue_5 "/Game/Niagara/Asteroids/Ice2.Ice2" (struct) (struct) true null))
            (:`then_2`
              (bind _returnvalue_6 (`self.MakeIceBall`))
              (`GeometryScriptLibrary_StaticMeshFunctions.CopyMeshToStaticMesh` _returnvalue_6 "/Game/Niagara/Asteroids/Ice3.Ice3" (struct) (struct) true null))
            (:`then_3`
              (bind _returnvalue_7 (`self.MakeIceBall`))
              (`GeometryScriptLibrary_StaticMeshFunctions.CopyMeshToStaticMesh` _returnvalue_7 "/Game/Niagara/Asteroids/Ice4.Ice4" (struct) (struct) true null))
            (:`then_4`
              (bind _returnvalue_8 (`self.MakeIceBall`))
              (`GeometryScriptLibrary_StaticMeshFunctions.CopyMeshToStaticMesh` _returnvalue_8 "/Game/Niagara/Asteroids/Ice5.Ice5" (struct) (struct) true null))))))
    (:`then_1`
      (for _array_element _comparray
        (`ActorComponent.K2_DestroyComponent` _array_element))
      (`KismetArrayLibrary.Array_Clear` _comparray))))

(fn `UserConstructionScript`)