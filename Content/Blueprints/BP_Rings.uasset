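; BP_Rings is an actor that builds a field of procedural asteroids at runtime, scattered through a spherical volume.
; On BeginPlay it adds dynamic mesh components with random rotations at random directions and distances within SpawnRadius, which clusters them toward the center.
; Each component gets the asteroid particle material, and AppendAsteroid fills its mesh using the shared AsteroidSettings and AsteroidScale.
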(event `self.ReceiveBeginPlay`
  (for _ (range (+ (`self.numAsteroids`) 1))
    (bind _returnvalue (`AddComponent|NODE_AddDynamicMeshComponent-2` :`RelativeTransform` (`KismetMathLibrary.MakeTransform` (* (`KismetMathLibrary.RandomUnitVector`) (* (`KismetMathLibrary.RandomFloat`) (`self.SpawnRadius`))) (`KismetMathLibrary.RandomRotator` false))))
    (`PrimitiveComponent.SetMaterial` _returnvalue 0 "/Game/Materials/M_AsteroidParticle.M_AsteroidParticle")
    (bind _returnvalue_2 (`BaseDynamicMeshComponent.GetDynamicMesh` _returnvalue))
    (`_JR_MeshFunctions.AppendAsteroid` _returnvalue_2 (`self.AsteroidSettings`) (`KismetMathLibrary.MakeTransform` (0.0 0.0 0.0) (struct) (`KismetMathLibrary.Conv_DoubleToVector` (`self.AsteroidScale`))))))

(fn `UserConstructionScript`)