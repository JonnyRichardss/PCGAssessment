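; Comet actor that orbits a sun at the world origin under simulated Newtonian gravity, configured through PlacementSettings.
; Construction randomly tilts the orbital plane, places the comet at its initial radius and generates a procedural ice-ball dynamic mesh.
; Tick integrates position, then velocity, on scaled time and derives eccentricity, periapsis and apoapsis for debugging.
; It also points Niagara ion and dust tails away from the origin, shortening the ion beam with distance.
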(event `self.ReceiveBeginPlay`
  (bind (_placementsettings_initialradius _placementsettings_initialvelocity) (break `CometPlacementSettings` (`self.PlacementSettings`)))
  (set `self.Velocity` (* _placementsettings_initialvelocity (`KismetMathLibrary.Normal` (`KismetMathLibrary.Cross_VectorVector` (`self.OrbitalPlane`) (`KismetMathLibrary.Normal` (`self.K2_GetActorLocation`)))))))

(event `self.ReceiveTick`
  (params (DeltaSeconds :type "Float (single-precision)"))
  (bind _returnvalue (`self.K2_GetActorLocation`))
  (bind (_placementsettings_initialradius _placementsettings_initialvelocity _placementsettings_size _placementsettings_mass _placementsettings_planedeviation _placementsettings_orbittimescale) (break `CometPlacementSettings` (`self.PlacementSettings`)))
  (bind (_placementsettings_initialradius_2 _placementsettings_initialvelocity_2 _placementsettings_size_2 _placementsettings_mass_2 _placementsettings_planedeviation_2 _placementsettings_orbittimescale_2 _placementsettings_ionlength _placementsettings_ionmaxdistance) (break `CometPlacementSettings` (`self.PlacementSettings`)))
  (bind (_placementsettings_initialradius_3 _placementsettings_initialvelocity_3 _placementsettings_size_3 _placementsettings_mass_3) (break `CometPlacementSettings` (`self.PlacementSettings`)))
  (bind (_placementsettings_initialradius_4 _placementsettings_initialvelocity_4 _placementsettings_size_4 _placementsettings_mass_4) (break `CometPlacementSettings` (`self.PlacementSettings`)))
  (bind _returnvalue_2 (* DeltaSeconds _placementsettings_orbittimescale))
  (bind _returnvalue_3 (- 1.0 (/ (`KismetMathLibrary.VSize` _returnvalue) _placementsettings_ionmaxdistance)))
  (`self.K2_SetActorLocation` (+ (* _returnvalue_2 (`self.Velocity`)) (`self.K2_GetActorLocation`)))
  (set `self.Velocity` (+ (`self.Velocity`) (* _returnvalue_2 (/ (`_JR_SolarSystemGenerator.NewtonGravity` _placementsettings_mass (`self.SolarMass`) (`self.K2_GetActorLocation`) (0.0 0.0 0.0)) _placementsettings_mass_3))))
  (`|ExecutionSequence`
    (:`then_0`
      ; Orbit Debug
      (bind _output_get (set `self.Mu` (* (+ _placementsettings_mass_4 (`self.SolarMass`)) (`_JR_SolarSystemGenerator.GetBigG`))))
      (bind _output_get_2 (set `self.SpE` (- (/ (`KismetMathLibrary.VSizeSquared` (`self.Velocity`)) 2.0) (/ _output_get (`KismetMathLibrary.VSize` (`self.K2_GetActorLocation`))))))
      (set `self.a` (/ (`self.Mu`) (* _output_get_2 -2.0)))
      (bind _output_get_3 (set `self.h` (`KismetMathLibrary.Cross_VectorVector` (`self.Velocity`) (`self.K2_GetActorLocation`))))
      (bind _output_get_4 (set `self.eccentricity` (`KismetMathLibrary.VSize` (- (/ (`KismetMathLibrary.Cross_VectorVector` (`self.Velocity`) _output_get_3) (`self.Mu`)) (`KismetMathLibrary.Normal` (`self.K2_GetActorLocation`))))))
      (set `self.Periapsis` (* (`self.a`) (- 1.0 _output_get_4)))
      (set `self.Apoapsis` (* (+ _output_get_4 1.0) (`self.a`))))
    (:`then_1`
      (`NiagaraComponent.SetVariableVec3` (`self.Niagara`) "Beam End" (* (`KismetMathLibrary.Normal` _returnvalue) (* (`KismetMathLibrary.SelectFloat` _returnvalue_3 0.0 (>= _returnvalue_3 0.0)) _placementsettings_ionlength)))
      (`NiagaraComponent.SetVariableVec3` (`self.DustTrail`) "Cone Axis" (`KismetMathLibrary.Normal` (`self.K2_GetActorLocation`))))))

(fn `UserConstructionScript`
  (bind _orbitalplane (`self.OrbitalPlane`))
  (bind (_placementsettings_initialradius _placementsettings_initialvelocity _placementsettings_size _placementsettings_mass _placementsettings_planedeviation _placementsettings_orbittimescale _placementsettings_ionlength _placementsettings_ionmaxdistance _placementsettings_generatorsettings) (break `CometPlacementSettings` (`self.PlacementSettings`)))
  (bind (_placementsettings_initialradius_2 _placementsettings_initialvelocity_2 _placementsettings_size_2 _placementsettings_mass_2 _placementsettings_planedeviation_2) (break `CometPlacementSettings` (`self.PlacementSettings`)))
  (bind (_icosphereiterations _basenoise) (break `IceBallSettings` _placementsettings_generatorsettings))
  (bind _returnvalue (`KismetMathLibrary.Normal` (`KismetMathLibrary.RotateAngleAxis` _orbitalplane _placementsettings_planedeviation_2 (`KismetMathLibrary.Cross_VectorVector` (`KismetMathLibrary.Normal` (`KismetMathLibrary.ProjectVectorOnToPlane` (`KismetMathLibrary.RandomUnitVector`) _orbitalplane)) _orbitalplane))))
  (set `self.OrbitalPlane` _returnvalue)
  (`self.K2_SetActorLocation` (* _placementsettings_initialradius_2 (`KismetMathLibrary.Normal` (`KismetMathLibrary.ProjectVectorOnToPlane` (`KismetMathLibrary.RandomUnitVector`) _returnvalue))))
  (bind _returnvalue_2 (`BaseDynamicMeshComponent.GetDynamicMesh` (`self.DynamicMesh`)))
  (`_JR_MeshFunctions.AppendIceBall` _returnvalue_2 (make `IceBallSettings` _icosphereiterations _basenoise) (`KismetMathLibrary.MakeTransform` (0.0 0.0 0.0) (struct) (`KismetMathLibrary.Conv_DoubleToVector` _placementsettings_size))))