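; BP_PlanetAtmo is a procedural planet actor with a land body and a water sphere, built in the construction script on dynamic mesh components.
; AppendPlanet generates the Body mesh from the planet settings and sea and land colors, shown through a vertex color material.
; An icosphere forms the Water mesh, with a dynamic material instance driven by sea color, shore color and shore size.
; The event graph has no active logic.
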(fn `UserConstructionScript`
  (bind _body (`self.Body`))
  (bind _water (`self.Water`))
  (`PrimitiveComponent.SetMaterial` _body 0 "/Game/Materials/VertexCol.VertexCol")
  (bind _returnvalue (`BaseDynamicMeshComponent.GetDynamicMesh` _body))
  (`_JR_MeshFunctions.AppendPlanet` _returnvalue (`self.Settings`) (`self.Transform`) (`KismetMathLibrary.Conv_LinearColorToVector` (`self.SeaCol`)) (`KismetMathLibrary.Conv_LinearColorToVector` (`self.LandCol`)))
  (bind _returnvalue_2 (`BaseDynamicMeshComponent.GetDynamicMesh` _water))
  (`_JR_MeshFunctions.AppendIcoSphere` _returnvalue_2 (`self.Transform`) 5)
  (bind _returnvalue_3 (`PrimitiveComponent.CreateDynamicMaterialInstance` _water 0 "/Game/Materials/waterMat.waterMat" "None"))
  (bind _output_get (set `self.WaterMat` _returnvalue_3))
  (`MaterialInstanceDynamic.SetVectorParameterValue` _output_get "BaseCol" (`self.SeaCol`))
  (`MaterialInstanceDynamic.SetVectorParameterValue` _output_get "EdgeCol" (`self.ShoreCol`))
  (`MaterialInstanceDynamic.SetScalarParameterValue` _output_get "EdgeSize" (`self.ShoreSize`)))