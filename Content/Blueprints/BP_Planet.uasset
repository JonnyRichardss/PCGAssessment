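; Procedural planet actor that builds itself from PlacementSettings and orbits the world origin while spinning about its orbital-plane normal.
; The construction script generates dynamic meshes and randomly coloured materials for Earth-like (with water sphere), gas giant or rocky types, optionally adding a BP_PlanetRing child actor.
; BeginPlay picks a random orbit position and tangential velocity, with optional debug circle.
; Tick manually integrates velocity and centripetal acceleration, scaled by orbit time scale.
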(event `self.ReceiveBeginPlay`
  (bind (_placementsettings_type _placementsettings_orbitradius) (break `PlanetPlacementSettings` (`self.PlacementSettings`)))
  (bind _orbitalplane (`self.OrbitalPlane`))
  (bind (_placementsettings_type_2 _placementsettings_orbitradius_2) (break `PlanetPlacementSettings` (`self.PlacementSettings`)))
  (bind (_placementsettings_type_3 _placementsettings_orbitradius_3 _placementsettings_planetsize _placementsettings_rotationspeed _placementsettings_bhasring _placementsettings_ringsettings _placementsettings_generationsettings _placementsettings_orbitspeed) (break `PlanetPlacementSettings` (`self.PlacementSettings`)))
  (bind _returnvalue (`KismetMathLibrary.Normal` (`KismetMathLibrary.ProjectVectorOnToPlane` (`KismetMathLibrary.RandomUnitVector`) _orbitalplane)))
  (`self.K2_SetActorLocation` (* (`KismetMathLibrary.Normal` (`KismetMathLibrary.ProjectVectorOnToPlane` (`KismetMathLibrary.RandomUnitVector`) (`self.OrbitalPlane`))) _placementsettings_orbitradius) false true)
  (`self.K2_AddActorWorldRotation` (`KismetMathLibrary.MakeRotFromZ` (`self.OrbitalPlane`)))
  (set `self.Velocity` (* _placementsettings_orbitspeed (`KismetMathLibrary.Normal` (`KismetMathLibrary.Cross_VectorVector` (`self.OrbitalPlane`) (`self.K2_GetActorLocation`)))))
  (if (`self.Debug`)
    (`KismetSystemLibrary.DrawDebugCircle` (0.0 0.0 0.0) _placementsettings_orbitradius_2 60 (struct :`R` 0.182907 :`G` 1.0 :`A` 1.0) 100000.0 1000.0 _returnvalue (`KismetMathLibrary.Cross_VectorVector` _returnvalue _orbitalplane))))

(event `self.ReceiveTick`
  (params (DeltaSeconds :type "Float (single-precision)"))
  (bind (_placementsettings_type _placementsettings_orbitradius _placementsettings_planetsize _placementsettings_rotationspeed _placementsettings_bhasring _placementsettings_ringsettings _placementsettings_generationsettings _placementsettings_orbitspeed _placementsettings_orbittimescale) (break `PlanetPlacementSettings` (`self.PlacementSettings`)))
  (bind _body (`self.Body`))
  (bind (_placementsettings_type_2 _placementsettings_orbitradius_2 _placementsettings_planetsize_2 _placementsettings_rotationspeed_2) (break `PlanetPlacementSettings` (`self.PlacementSettings`)))
  (bind _returnvalue (* DeltaSeconds _placementsettings_orbittimescale))
  (`self.K2_SetActorLocation` (+ (* _returnvalue (`self.Velocity`)) (`self.K2_GetActorLocation`)))
  (set `self.Velocity` (+ (`self.Velocity`) (* _returnvalue (`KismetMathLibrary.Normal` (`self.K2_GetActorLocation`)) (`KismetMathLibrary.Conv_DoubleToVector` -1.0) (/ (`KismetMathLibrary.VSizeSquared` (`self.Velocity`)) (`KismetMathLibrary.VSize` (`self.K2_GetActorLocation`))))))
  (`SceneComponent.K2_SetWorldRotation` _body (`KismetMathLibrary.ComposeRotators` (`SceneComponent.K2_GetComponentRotation` _body) (`KismetMathLibrary.RotatorFromAxisAndAngle` (`self.OrbitalPlane`) (+ 0.0 (* (`GameplayStatics.GetWorldDeltaSeconds`) _placementsettings_rotationspeed_2)))) false false))

(fn `RandomColour`
  (returns (Colour :type "LinearColor Structure"))
  (return (`KismetMathLibrary.MakeColor` (`KismetMathLibrary.RandomFloat`) (`KismetMathLibrary.RandomFloat`) (`KismetMathLibrary.RandomFloat`))))

(fn `UserConstructionScript`
  (bind _colour (`self.RandomColour`))
  (bind (_placementsettings_type _placementsettings_orbitradius _placementsettings_planetsize _placementsettings_rotationspeed _placementsettings_bhasring _placementsettings_ringsettings) (break `PlanetPlacementSettings` (`self.PlacementSettings`)))
  (bind (_placementsettings_type_2 _placementsettings_orbitradius_2 _placementsettings_planetsize_2 _placementsettings_rotationspeed_2 _placementsettings_bhasring_2) (break `PlanetPlacementSettings` (`self.PlacementSettings`)))
  (bind _placementsettings_type_3 (break `PlanetPlacementSettings` (`self.PlacementSettings`)))
  (bind (_placementsettings_type_4 _placementsettings_orbitradius_3 _placementsettings_planetsize_3 _placementsettings_rotationspeed_3 _placementsettings_bhasring_3 _placementsettings_ringsettings_2 _placementsettings_generationsettings) (break `PlanetPlacementSettings` (`self.PlacementSettings`)))
  (bind _water (`self.Water`))
  (bind _body (`self.Body`))
  (bind (_transform_location _transform_rotation _transform_scale) (`KismetMathLibrary.BreakTransform` (`self.Transform`)))
  (bind (_placementsettings_type_5 _placementsettings_orbitradius_4 _placementsettings_planetsize_4 _placementsettings_rotationspeed_4 _placementsettings_bhasring_4 _placementsettings_ringsettings_3 _placementsettings_generationsettings_2) (break `PlanetPlacementSettings` (`self.PlacementSettings`)))
  ; Init
  (`|ExecutionSequence`
    (:`then_1`
      (set `self.Transform` (`KismetMathLibrary.MakeTransform` (0.0 0.0 0.0) (struct) (`KismetMathLibrary.Conv_DoubleToVector` _placementsettings_planetsize_4)))
      (set `self.Settings` _placementsettings_generationsettings_2)
      (switch `PlanetType` _placementsettings_type_3
        (:`EarthLike`
          ; ELW
          (`PrimitiveComponent.SetMaterial` _body 0 "/Game/Materials/VertexCol.VertexCol")
          (bind _returnvalue (`BaseDynamicMeshComponent.GetDynamicMesh` _body))
          (`_JR_MeshFunctions.AppendEarthPlanet` _returnvalue (`self.Settings`) (`self.Transform`) (`KismetMathLibrary.Conv_LinearColorToVector` _colour) (`KismetMathLibrary.Conv_LinearColorToVector` (`self.RandomColour`)))
          (bind _returnvalue_2 (`BaseDynamicMeshComponent.GetDynamicMesh` _water))
          (bind _returnvalue_3 (`_JR_MeshFunctions.AppendIcoSphere` _returnvalue_2 (`self.Transform`) 5))
          (`GeometryScriptLibrary_MeshNormalsFunctions.RecomputeNormals` _returnvalue_3 (struct) false null)
          (bind _returnvalue_4 (`PrimitiveComponent.CreateDynamicMaterialInstance` _water 0 "/Game/Materials/waterMat.waterMat" "None"))
          (`MaterialInstanceDynamic.SetVectorParameterValue` _returnvalue_4 "BaseCol" _colour)
          (`MaterialInstanceDynamic.SetVectorParameterValue` _returnvalue_4 "EdgeCol" (`self.RandomColour`))
          (`MaterialInstanceDynamic.SetScalarParameterValue` _returnvalue_4 "EdgeSize" 80.0)
          ; Ring
          (if _placementsettings_bhasring_2 :!label _label
            (bind _returnvalue_5 (`AddComponent|NODE_AddChildActorComponent-0`))
            (`ChildActorComponent.SetChildActorClass` _returnvalue_5 "/Game/Blueprints/BP_PlanetRing.BP_PlanetRing_C")
            (bind _asbp_planet_ring (cast `/Game/Blueprints/BP_PlanetRing` (`ChildActorComponent.ChildActor` _returnvalue_5))
              (:`then`
                (set `/Game/Blueprints/BP_PlanetRing.RingSettings` _placementsettings_ringsettings _asbp_planet_ring))
              (:`CastFailed`
                (`KismetSystemLibrary.PrintString` "FAILED TO CAST RING TO RING LOL")))))
        (:`GasGiant`
          ; GAS
          (`ActorComponent.K2_DestroyComponent` (`self.Water`))
          (bind _returnvalue_6 (`BaseDynamicMeshComponent.GetDynamicMesh` (`self.Body`)))
          (bind _returnvalue_7 (`_JR_MeshFunctions.AppendIcoSphere` _returnvalue_6 (`self.Transform`) (`.icoSphereIterations` (break `PlanetSettings` _placementsettings_generationsettings))))
          (`GeometryScriptLibrary_MeshNormalsFunctions.RecomputeNormals` _returnvalue_7 (struct) false null)
          (bind _returnvalue_8 (`PrimitiveComponent.CreateDynamicMaterialInstance` (`self.Body`) 0 "/Game/Materials/M_GasGiant.M_GasGiant" "None"))
          (`MaterialInstanceDynamic.SetScalarParameterValue` _returnvalue_8 "Scale" (/ 10.0 (.x _transform_scale)))
          (`|ExecutionSequence`
            (:`then_0`
              (`MaterialInstanceDynamic.SetVectorParameterValue` _returnvalue_8 "Col1" (`self.RandomColour`)))
            (:`then_1`
              (`MaterialInstanceDynamic.SetVectorParameterValue` _returnvalue_8 "Col2" (`self.RandomColour`)))
            (:`then_2`
              (`MaterialInstanceDynamic.SetVectorParameterValue` _returnvalue_8 "Col3" (`self.RandomColour`)))
            (:`then_3`
              (goto _label))))
        (:`Rocky`
          ; ROCK
          (`ActorComponent.K2_DestroyComponent` (`self.Water`))
          (bind _returnvalue_9 (`BaseDynamicMeshComponent.GetDynamicMesh` (`self.Body`)))
          (`_JR_MeshFunctions.AppendRockPlanet` _returnvalue_9 (`self.Settings`) (`self.Transform`) (0.0 0.0 0.0) (1.0 1.0 1.0))
          (bind _returnvalue_10 (`PrimitiveComponent.CreateDynamicMaterialInstance` (`self.Body`) 0 "/Game/Materials/M_RockyPlanet.M_RockyPlanet" "None"))
          (`MaterialInstanceDynamic.SetVectorParameterValue` _returnvalue_10 "LowCol" (`self.RandomColour`))
          (`MaterialInstanceDynamic.SetVectorParameterValue` _returnvalue_10 "HiCol" (`self.RandomColour`))
          (goto _label))))))