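; BP_PlanetRing is a planetary ring actor that configures a Niagara ring of rocks from its RingSettings.
; On BeginPlay it scales the actor by orbit radius, pushes coverage, radius, count, rotation speed and rock scale into the system, then resets it.
; It adds a world rotation built from OrbitPlane as the Z axis, taking that plane from RingSettings unless DontRotate is set.
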(event `self.ReceiveBeginPlay`
  (bind (_ringsettings_orbitradius _ringsettings_disccoverage _ringsettings_ringradius _ringsettings_spawncount _ringsettings_maxrotationspeed _ringsettings_rockscale _ringsettings_orbitplane) (break `RingSettings` (`self.RingSettings`)))
  (bind _planetring (`self.PlanetRing`))
  (`self.SetActorScale3D` (`KismetMathLibrary.Conv_DoubleToVector` _ringsettings_orbitradius))
  (`NiagaraComponent.SetVariableFloat` _planetring "Disc Coverage" _ringsettings_disccoverage)
  (`NiagaraComponent.SetVariableFloat` _planetring "Ring Radius" _ringsettings_ringradius)
  (`NiagaraComponent.SetVariableInt` _planetring "Spawn Count" _ringsettings_spawncount)
  (`NiagaraComponent.SetVariableFloat` _planetring "MaxRotationSpeed" _ringsettings_maxrotationspeed)
  (`NiagaraComponent.SetVariableFloat` _planetring "ScaleMult" _ringsettings_rockscale)
  (`NiagaraComponent.ResetSystem` _planetring)
  (if (not (`self.DontRotate`))
    (set `self.OrbitPlane` _ringsettings_orbitplane))
  (`self.K2_AddActorWorldRotation` (`KismetMathLibrary.MakeRotFromZ` (`self.OrbitPlane`))))

(fn `UserConstructionScript`)