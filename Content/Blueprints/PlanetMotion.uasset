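; PlanetMotion is an actor Blueprint that moves itself along a circular orbit every Tick.
; Sine and cosine of game time times OrbitSpeed, in degrees, give X and Y, scaled by RadiusMultiplier along with a constant Z offset.
; The result is an absolute, swept location around the world origin, keeping rotation and scale.
; An unconnected variant that adds the current location is left unused.
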(event `self.ReceiveBeginPlay`)

(event `self.ReceiveTick`
  (params (DeltaSeconds :type "Float (single-precision)"))
  (bind _returnvalue (* (`KismetSystemLibrary.GetGameTimeInSeconds`) (`self.OrbitSpeed`)))
  (`self.K2_SetActorTransform` (`KismetMathLibrary.MakeTransform` (* (`self.RadiusMultiplier`) (`KismetMathLibrary.MakeVector` (`KismetMathLibrary.DegSin` _returnvalue) (`KismetMathLibrary.DegCos` _returnvalue) 0.5)) (.rotation (`self.GetTransform`)) (.scale (`self.GetTransform`))) true))

(fn `UserConstructionScript`)