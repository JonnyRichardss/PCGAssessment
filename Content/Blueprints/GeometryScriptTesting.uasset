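; GeometryScriptTesting is a test Blueprint for procedurally generated meshes, built on the generated dynamic mesh rebuild event.
; On rebuild it appends an ice ball to the target mesh using its ice ball settings and a transform.
; Disconnected calls for appending an asteroid or planet and making a system from a template remain in the graph but never run.
; BeginPlay, Tick, overlap and the construction script do nothing.
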(event `self.ReceiveBeginPlay`)

(event `self.OnRebuildGeneratedMesh`
  (params (TargetMesh :type "DynamicMesh Object Reference"))
  (`_JR_MeshFunctions.AppendIceBall` TargetMesh (`self.IceBallSettings`) (`self.Transform`)))

(fn `UserConstructionScript`)