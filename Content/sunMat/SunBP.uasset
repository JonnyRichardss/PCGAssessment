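; Sun actor Blueprint that shows a swappable material on its ShapeSphere mesh.
; BeginPlay applies SunMat to the sphere.
; NextMat increments CurrentMat, wraps it by modulo of the Mats array's last index and applies that entry, so the final material is never selected.
; Nothing in this Blueprint calls NextMat.
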(event `self.ReceiveBeginPlay`
  (`PrimitiveComponent.SetMaterial` (`self.Shape_Sphere`) 0 "/Game/sunMat/SunMat.SunMat"))

(fn `NextMat`
  (bind _result (`/Engine/EditorBlueprintResources/StandardMacros.IncrementInt` (`self.currentMat`))
    (:`  `
      (bind _output_get (set `self.currentMat` (mod _result (`KismetArrayLibrary.Array_LastIndex` (`self.Mats`)))))
      (`PrimitiveComponent.SetMaterial` (`self.Shape_Sphere`) 0 (`|GetArrayItem` (`self.Mats`) _output_get)))))

(fn `UserConstructionScript`)